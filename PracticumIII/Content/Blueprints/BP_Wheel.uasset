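; BP_Wheel is an interactable wheel that plays the WheelRotate level sequence when the player uses E nearby.
; Overlap of its Box by BP_ThirdPersonCharacter opens a Gate, and end overlap closes it.
; Both press and release of E enter that Gate, and a DoOnce behind it lets the sequence player be created and played only once.
; Debug strings print along the way.
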(event OnComponentBeginOverlap(Box)
  (params (OverlappedComponent :type Primitive%20Component%20Object%20Reference) (OtherActor :type Actor%20Object%20Reference) (OtherComp :type Primitive%20Component%20Object%20Reference) (OtherBodyIndex :type Integer) (bFromSweep :type Boolean) (SweepResult :type Hit%20Result%20Structure%20%28by%20ref%29))
  (Utilities|Casting|CastToBP_ThirdPersonCharacter OtherActor)
  (Development|PrintString "Player found")
  (Utilities|FlowControl|Gate true) ; enters at Open
)

(event OnComponentEndOverlap(Box)
  (params (OverlappedComponent :type Primitive%20Component%20Object%20Reference) (OtherActor :type Actor%20Object%20Reference) (OtherComp :type Primitive%20Component%20Object%20Reference) (OtherBodyIndex :type Integer))
  (Utilities|Casting|CastToBP_ThirdPersonCharacter OtherActor)
  (Utilities|FlowControl|Gate true) ; enters at Close
)

(event EventBeginPlay)

(event EventTick
  (params (DeltaSeconds :type Float%20%28single-precision%29)))

(event Input|KeyboardEvents|E
  (params (Key :type Key%20Structure :default "None"))
  (:Pressed
    (Development|PrintString "E pressed" :!label _label)
    (Utilities|FlowControl|Gate true
      (:Exit
        (Development|PrintString "Gate Opened")
        (Utilities|FlowControl|DoOnce false
          (:Completed
            (bind _outactor (Sequencer|Player|CreateLevelSequencePlayer "/Game/Sequences/WheelRotate.WheelRotate"))
            (Sequencer|Player|Play (Variables|/Script/LevelSequence.LevelSequenceActor|GetSequencePlayer _outactor) :!class /Script/MovieScene.MovieSceneSequencePlayer))))))
  (:Released
    (goto _label)))

(fn ConstructionScript)